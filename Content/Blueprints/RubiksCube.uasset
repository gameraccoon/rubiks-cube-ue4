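; RubiksCube actor that builds a centered 3D grid of static mesh pieces in the Construction Script, with no gameplay logic.
; Nested loops over XSize, YSize and ZSize add one mesh component per cell, placed by CalcLocation.
; CalcPos spaces each axis at a fixed distance, minus the ResetToCenter half-extent.
; The X and Z loop indices are passed swapped, so centering holds only when XSize equals ZSize.
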(event EventBeginPlay)

(event EventActorBeginOverlap
  (params (OtherActor :type Actor%20Object%20Reference)))

(event EventTick
  (params (DeltaSeconds :type Float%20%28single-precision%29)))

(fn ConstructionScript
  (for _index (range 0 (- (Variables|Parameters|GetxSize) 1))
    (for _index_2 (range 0 (- (Variables|Parameters|GetySize) 1))
      (for _index_3 (range 0 (- (Variables|Parameters|GetzSize) 1))
        (AddComponent|AddStaticMeshComponent false (Math|Transform|MakeTransform (Utilities|CalcLocation _index_3 _index_2 _index)))))))